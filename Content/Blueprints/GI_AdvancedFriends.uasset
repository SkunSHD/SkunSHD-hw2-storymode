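; Game instance Blueprint that handles multiplayer session hosting, joining and map travel through Advanced Sessions.
; Hosting creates a ten-player session, then opens the Lobby level as a listen server; a separate event runs servertravel to MapName.
; Joining searches all server types and, after looping through the results with an empty body, joins the last element.
; Accepted session invites join the invited session directly.
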(event `TravelServer`
  (`KismetSystemLibrary.ExecuteConsoleCommand` (`KismetStringLibrary.Concat_StrStr` "servertravel " (`self.MapName`)) null))

(event `Host Session`
  (`CreateSessionCallbackProxyAdvanced.CreateAdvancedSession` :`PlayerController` (`GameplayStatics.GetPlayerController` 0) :`PublicConnections` 10
    (:`OnSuccess`
      (`GameplayStatics.OpenLevel` "Lobby" true "listen"))))

(event `Join Session`
  (bind _results (`FindSessionsCallbackProxyAdvanced.FindSessionsAdvanced` (`GameplayStatics.GetPlayerController` 0) 0 false "AllServers")
    (:`OnSuccess`
      (for _array_element _results
        _)
      (`JoinSessionCallbackProxy.JoinSession` (`GameplayStatics.GetPlayerController` 0) _array_element))))

(event `self.OnSessionInviteAccepted`
  (params (LocalPlayerNum :type Integer) (PersonInvited :type "BPUniqueNetId Structure") (SessionToJoin :type "BlueprintSessionResult Structure (by ref)"))
  (`JoinSessionCallbackProxy.JoinSession` (`GameplayStatics.GetPlayerController` 0) SessionToJoin))