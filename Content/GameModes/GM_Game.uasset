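; GM_Game is the game mode for a team-based match with attacker and defender sides.
; On BeginPlay it caches all AttackerSpawn and DefenderSpawn actors, and on PostLogin it messages each new player to show team selection.
; SpawnAttacker and SpawnDefender pick a random spawn point for the side and message the controller to spawn the matching character there.
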(event Custom|SpawnAttacker
  (params (Controller :type Player%20Controller%20Object%20Reference))
  (Class|INTPCGame|SpawnPlayer(Message) Controller "/Game/Characters/B_CharacterAttacker.B_CharacterAttacker_C" (CallFunction|GetRandomPositionTransform (Variables|Default|GetAttackerSpawnPoints))))

(event Custom|SpawnDefender
  (params (Controller :type Player%20Controller%20Object%20Reference))
  (Class|INTPCGame|SpawnPlayer(Message) Controller "/Game/Characters/B_CharacterDefender.B_CharacterDefender_C" (CallFunction|GetRandomPositionTransform (Variables|Default|GetDefenderSpawnPoints))))

(event EventBeginPlay
  ;[1 1 1] Store Spawn Points
  (Utilities|FlowControl|Sequence
    (:then_0
      (bind _outactors (Actor|GetAllActorsOfClass "/Game/Blueprints/AttackerSpawn.AttackerSpawn_C"))
      (Variables|Default|SetAttackerSpawnPoints _outactors))
    (:then_1
      (bind _outactors_2 (Actor|GetAllActorsOfClass "/Game/Blueprints/DefenderSpawn.DefenderSpawn_C"))
      (Variables|Default|SetDefenderSpawnPoints _outactors_2))))

(event EventPostLogin
  (params (NewPlayer :type Player%20Controller%20Object%20Reference))
  (Class|INTPCGame|ShowTeamSelection(Message) NewPlayer))

(fn ConstructionScript)

(fn GetRandomPositionTransform
  (params (Positions :type Array%20of%20Player%20Start%20Object%20References))
  (return (Transformation|GetActorTransform (Utilities|Array|Get(acopy) Positions (Math|Random|RandomIntegerinRange 0 (- (Utilities|Array|Length Positions) 1))))))