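; PC_Game is the game's player controller, handling team selection and spawning as attacker or defender.
; It shows the team selection widget with cursor and UI input over a tagged level camera.
; Attacker and defender requests pass through Server-named events to GM_Game's spawn functions.
; SpawnPlayer spawns and possesses the given character, then calls for widget removal, whose Client-named event restores game-only input.
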(event Custom|ServerAttackerSpawn
  (Default|SpawnAttacker (Variables|Default|GetGameMode) self))

(event Custom|ServerDefenderSpawn
  (Default|SpawnDefender (Variables|Default|GetGameMode) self))

(event Custom|ClientShowTeamSelection
  (bind _returnvalue (UserInterface|CreateWidget "/Game/Widgets/W_SelectTeam.W_SelectTeam_C"))
  (bind _output_get (Variables|Default|SetTeamSelectionWidget _returnvalue))
  (UserInterface|Viewport|AddtoViewport _output_get 0)
  (Input|SetInputModeGameandUI self (Variables|Default|GetTeamSelectionWidget) "DoNotLock" true)
  (Variables|Default|SetbShowMouseCursor true)
  ;[1 1 1] Setup Level Camera
  (bind _outactors (Actor|GetAllActorsOfClasswithTag "/Script/Engine.CameraActor" "DefaultLevelCamera"))
  (if (> (Utilities|Array|Length _outactors) 0)
    (Game|Player|SetViewTargetwithBlend (Utilities|Array|Get(acopy) _outactors) 0.0 "VTBlend_Linear" 0.0 false)))

(event Custom|Client_RemoveTeamSelectionWidget
  (Widget|RemovefromParent (Variables|Default|GetTeamSelectionWidget))
  (Input|SetInputModeGameOnly self)
  (Variables|Default|SetbShowMouseCursor false))

(event EventBeginPlay
  ;[1 1 1] Store GameMode
  (bind _asgm_game (Utilities|Casting|CastToGM_Game (Game|GetGameMode)))
  (Variables|Default|SetGameMode _asgm_game))

(event EventAttackerSpawn
  (CallFunction|ServerAttackerSpawn))

(event EventDefenderSpawn
  (CallFunction|ServerDefenderSpawn))

(event EventShowTeamSelection
  (CallFunction|ClientShowTeamSelection))

(event EventSpawnPlayer
  (params (Character :type Character%20Class%20Reference) (Transform :type Transform))
  (bind _returnvalue (Game|SpawnActorfromClass Character Transform "AdjustIfPossibleButAlwaysSpawn" 0 0))
  (Pawn|Possess _returnvalue)
  (CallFunction|ClientRemoveTeamSelectionWidget))

(fn ConstructionScript)